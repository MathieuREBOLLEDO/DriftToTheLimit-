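; Test player car pawn for an arcade racer with drift and nitro, moved by setting location and rotation directly rather than by physics.
; Timelines sampled through float curves drive acceleration, deceleration and nitro speed, while drifting with steering fills the Energy that nitro spends.
; Downward traces keep a minimum ground height, align rotation to the surface and apply manual gravity in the air.
; Hits redirect the car along walls; BeginPlay spawns HUD, debug and editor widgets.
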(event `CheckFront`
  (bind _returnvalue (`SceneComponent.K2_GetComponentLocation` (`self.RearCar`)))
  (bind _returnvalue_2 (`SceneComponent.K2_GetComponentLocation` (`self.Front Car`)))
  ;[0 0.2423 0] Check ground
  (`|ExecutionSequence`
    (:`then_0`
      ;;[1 1 1] Front Check
      (bind (_outhit _returnvalue_3) (`KismetSystemLibrary.LineTraceSingle` :`Start` _returnvalue_2 :`End` (+ _returnvalue_2 (* (`KismetMathLibrary.NegateVector` (`self.GetActorUpVector`)) 200.0)) :`TraceChannel` "TraceTypeQuery1" :`DrawDebugType` (select `bool` (`self.isDebug`) :`true` "ForDuration" :!type "EDrawDebugTrace Enum") :`TraceColor` (struct :`R` 0.143653 :`B` 1.0 :`A` 1.0)))
      (set `self.FrontOnGround` _returnvalue_3))
    (:`then_1`
      ;;[1 1 1] Rear Check
      (bind (_outhit_2 _returnvalue_4) (`KismetSystemLibrary.LineTraceSingle` :`Start` _returnvalue :`End` (+ _returnvalue (* (`KismetMathLibrary.NegateVector` (`self.GetActorUpVector`)) 200.0)) :`TraceChannel` "TraceTypeQuery1" :`DrawDebugType` (select `bool` (`self.isDebug`) :`true` "ForDuration" :!type "EDrawDebugTrace Enum") :`TraceColor` (struct :`G` 1.0 :`B` 0.706942 :`A` 1.0)))
      (set `self.RearOnGround` _returnvalue_4)))
  (set `self.isOnGround` (and (`self.FrontOnGround`) (`self.RearOnGround`))))

(event `self.ReceiveBeginPlay`
  ;[1 1 1] Begin Play
  (set `self.CurrentSpeed` (`self.MAXSpeed`))
  (set `self.RestartPos` (`self.GetTransform`))
  (`KismetSystemLibrary.K2_SetTimerDelegate` (delegate `Update`) 0.25 true)
  ;;[1 0.5 0] HUD
  (bind _returnvalue (`|CreateWidget` "/Game/Root/GD/Player/Widget/WB_HUD.WB_HUD_C"))
  (`UserWidget.AddToViewport` _returnvalue 0)
  ;;[1 0.5 0] Debug Widget
  (`self.SetWidget Debug`)
  ;;[1 0.5 0] Editor Widget
  (`self.SetWidget Editor`)
  (`KismetSystemLibrary.K2_SetTimerDelegate` (delegate `CheckFront`) 0.15 true))

(event `self.ReceiveHit`
  (params (MyComp :type "PrimitiveComponent Object Reference") (Other :type "Actor Object Reference") (OtherComp :type "PrimitiveComponent Object Reference") (bSelfMoved :type Boolean) (HitLocation :type "Vector Structure") (HitNormal :type "Vector Structure") (NormalImpulse :type "Vector Structure") (Hit :type "HitResult Structure (by ref)"))
  (bind _returnvalue (`self.GetActorForwardVector`))
  (bind (_bblockinghit _binitialoverlap _time _distance _location _impactpoint _normal) (`GameplayStatics.BreakHitResult` Hit))
  (bind (_returnvalue_x _returnvalue_y _returnvalue_z) (`KismetMathLibrary.BreakVector` (`KismetMathLibrary.Cross_VectorVector` (`self.GetActorForwardVector`) _normal)))
  (bind _returnvalue_2 (select `bool` (`self.isDebug`) :`true` "ForDuration" :!type "EDrawDebugTrace Enum"))
  ;[0 1 1] Collision
  (`KismetSystemLibrary.LineTraceSingle` :`Start` HitLocation :`End` (+ HitLocation (* _normal 500.0)) :`TraceChannel` "TraceTypeQuery1" :`bTraceComplex` true :`DrawDebugType` _returnvalue_2)
  (`KismetSystemLibrary.LineTraceSingle` :`Start` HitLocation :`End` (+ HitLocation (* (`KismetMathLibrary.MirrorVectorByNormal` (`self.GetActorForwardVector`) _normal) 500.0)) :`TraceChannel` "TraceTypeQuery1" :`bTraceComplex` true :`DrawDebugType` _returnvalue_2)
  (`self.K2_SetActorRotation` (`KismetMathLibrary.ComposeRotators` (`KismetMathLibrary.FindLookAtRotation` _returnvalue (`KismetMathLibrary.ProjectVectorOnToPlane` _returnvalue _normal)) (`KismetMathLibrary.RotatorFromAxisAndAngle` (`self.GetActorUpVector`) (select `bool` (< _returnvalue_z 0.0) :`false` -90.0 :`true` 90.0 :!type "Float (single-precision)")))))

(event `ResetAccTime`
  ;[1 1 1] Update
  ;;[0 1 0] Start Update Acc
  (bind _output_get (set `self.ScaleAccCurve` (select `bool` (`self.DecIsOver`) :`false` (- 1.0 (`self.ScaleDecCurve`)) :!type "Float (single-precision)") :!label _label))
  (bind (_direction _time) (`Timeline|UpdateAccTime` :`NewTime` _output_get :!via `SetNewTime` :!label _label_2)
    (:`Update`
      (set `self.ScaleAccCurve` _time))))

(event `Update`
  ;[1 1 1] Update
  ;;[0.5 0 0.5] Seting Timer Value
  (`TimelineComponent.SetPlayRate` (`self.UpdateAccTime`) (/ 1.0 (`self.AccTime`)))
  (`TimelineComponent.SetPlayRate` (`self.UpdateDecelerationTime`) (/ 1.0 (`self.DecTime`)))
  (`TimelineComponent.SetPlayRate` (`self.UpdateNitroTime`) (/ 1.0 (`self.NitroTime`)))
  (`|ExecutionSequence`
    (:`then_0`
      ;;[0 1 0] Start Update Acc
      (if (`self.IsAccelerating`)
        (set `self.Acc_Released` false)
        (`self.ResetDecTime`)
        (goto _label_2)
        (else
          (goto _label))))
    (:`then_1`
      ;;[0 1 0] Update Deceleration
      (if (and (`self.Acc_Released`) (not (`self.isNitro`)))
        (bind (_direction _time) (`Timeline|UpdateDecelerationTime` :!label _label_3)
          (:`Update`
            (set `self.ScaleDecCurve` _time)
            (set `self.DecIsOver` false))
          (:`Finished`
            (`self.ResetAccTime`)
            (set `self.Acc_Released` false)
            (`self.ResetDecTime`)
            (set `self.DecIsOver` true)
            (set `self.LastSpeed` 0.0)))
        (else
          (goto _label_3 :!via `Stop`))))
    (:`then_2`
      ;;[1 1 0] Nitro
      (if (`self.isNitro`)
        (bind (_direction_2 _time_2) (`Timeline|UpdateNitroTime` :!label _label_4)
          (:`Update`
            (set `self.ScaleNitro` _time_2))
          (:`Finished`
            (`self.Reset Nitro Time`)
            (set `self.isNitro` false)
            (set `self.Energy` 0.0)))
        (else
          (goto _label_4 :!via `Stop`))))))

(event `ResetDecTime`
  ;[1 1 1] Update
  ;;[0 1 0] Update Deceleration
  (goto _label_3 :!via `SetNewTime`))

(event `Reset Nitro Time`
  ;[1 1 1] Update
  ;;[1 1 0] Nitro
  (goto _label_4 :!via `SetNewTime`))

(event `Key|R`
  (params (Key :type "Key Structure"))
  ;[1 1 1] Input
  (:`Pressed`
    (`self.K2_SetActorTransform` (`self.RestartPos`))))

(event `InputAction|Acceleration`
  (params (Key :type "Key Structure"))
  ;[1 1 1] Input
  ;;[0 1 0] Acc & Dec
  (:`Pressed`
    (if (not (`self.isNitro`))
      (set `self.IsAccelerating` true)))
  (:`Released`
    (set `self.IsAccelerating` false)
    (set `self.Acc_Released` true)))

(event `InputAxis|Throttle`
  (params (AxisValue :type "Float (single-precision)"))
  ;[1 1 1] Input
  ;;[0 0 0] Basic Throttle
)

(event `InputAxis|Sterring`
  (params (AxisValue :type "Float (single-precision)"))
  ;[1 1 1] Input
  ;;[0 0.2232 0.3916] Basic Sterring
  (if (`self.IsDrifting`)
    (if (== (`self.DriftDirection`) 0)
      (set `self.DriftDirection` (`KismetMathLibrary.FTrunc` AxisValue)))
    (else
      (set `self.IsSterring` (!= AxisValue 0.0))
      (`self.K2_SetActorRotation` (`KismetMathLibrary.ComposeRotators` (`self.K2_GetActorRotation`) (`KismetMathLibrary.RotatorFromAxisAndAngle` (`self.GetActorUpVector`) (* AxisValue (`self.SterringSpeed`))))))))

(event `self.ReceiveTick`
  (params (DeltaSeconds :type "Float (single-precision)"))
  (bind _returnvalue (`self.K2_GetActorLocation`))
  (bind (_returnvalue_x _returnvalue_y _returnvalue_z) (`KismetMathLibrary.BreakVector` (`self.K2_GetActorLocation`)))
  ;[1 1 1] Event Tick
  (`|ExecutionSequence`
    (:`then_0`
      (`SceneComponent.SetHiddenInGame` (`self.CarBase`) (not (`self.isDebug`)) false)
      (if (`self.isDebug`)
        (`self.Debug`)))
    (:`then_2`
      ;;[1 1 0] Boost Nitro
      (if (`self.isNitro`)
        (`self.K2_SetActorLocation` (+ (`self.K2_GetActorLocation`) (* (`KismetMathLibrary.MapRangeClamped` (`CurveFloat.GetFloatValue` (`self.NitroCurve`) (`self.ScaleNitro`)) 0.0 1.0 (`self.LastSpeed`) (`self.NitroSpeed`)) (`self.GetActorForwardVector`))) true)
        ;;[1 1 0] Set Energy during Nitro
        ;;;[1 0 0] Bug of nitro Speed
        (set `self.Energy` (`KismetMathLibrary.MapRangeClamped` (`self.ScaleNitro`) 0.0 1.0 (`self.EnergyBeforeNitro`)))))
    (:`then_3`
      ;;[0 1 0] Acceleration
      (if (`self.IsAccelerating`)
        (`self.K2_SetActorLocation` (+ (`self.K2_GetActorLocation`) (* (`self.MAXSpeed`) (`CurveFloat.GetFloatValue` (`self.AccCurve`) (`self.ScaleAccCurve`)) (`self.GetActorForwardVector`))) true)
        (else
          ;;[0 1 0] Deceleration
          (if (`self.Acc_Released`)
            (`self.K2_SetActorLocation` (+ (`self.K2_GetActorLocation`) (* (`self.MAXSpeed`) (`CurveFloat.GetFloatValue` (`self.DecCurve`) (`self.ScaleDecCurve`)) (`self.GetActorForwardVector`))) true)))))
    (:`then_5`
      ;;[0 0.09759 0] Put player at a minimun distance of the ground if player goes under
      (bind _outhit (`KismetSystemLibrary.LineTraceSingle` :`Start` _returnvalue :`End` (+ _returnvalue (* (`KismetMathLibrary.NegateVector` (`self.GetActorUpVector`)) 500.0)) :`TraceChannel` "TraceTypeQuery1" :`DrawDebugType` (select `bool` (`self.isDebug`) :`true` "ForDuration" :!type "EDrawDebugTrace Enum")))
      (bind (_bblockinghit _binitialoverlap _time _distance _location) (`GameplayStatics.BreakHitResult` _outhit))
      (bind _returnvalue_2 (`KismetMathLibrary.VSize` (- _returnvalue _location)))
      (if (or (< _returnvalue_2 (`self.minDistanceToGround`)) (< _returnvalue_2 (+ (`self.minDistanceToGround`) 50.0)))
        (`self.K2_SetActorLocation` (+ _location (* (`self.GetActorUpVector`) (`self.minDistanceToGround`))) true)
        ;;[0 1 1] Update Rot from Ground
        ;;;[1 1 1] On Ground
        (if (`self.isOnGround`)
          (bind _newrotation (`self.UpdateRotToGround` 500.0 (`self.GetActorUpVector`)))
          (`self.K2_SetActorRotation` (`KismetMathLibrary.RInterpTo` (`self.K2_GetActorRotation`) _newrotation (`GameplayStatics.GetWorldDeltaSeconds`) 10.0)))
        (else
          ;;;[0 0.2423 0] Gravity
          (if (not (`self.RearOnGround`))
            (`self.K2_SetActorLocation` (`KismetMathLibrary.MakeVector` _returnvalue_x _returnvalue_y (- _returnvalue_z (`self.Gravity`))) true)
            ;;;[1 1 1] In Air
            (bind _newrotation_2 (`self.UpdateRotToGround` 5000.0 (`KismetMathLibrary.Vector_Up`)))
            (`self.K2_SetActorRotation` (`KismetMathLibrary.RInterpTo` (`self.K2_GetActorRotation`) _newrotation_2 (`GameplayStatics.GetWorldDeltaSeconds`) 8.0))))))))

(event `InputAxis|Drift`
  (params (AxisValue :type "Float (single-precision)"))
  ;[1 1 1] Input
  ;;[1 0 1] Basic Drift
  (bind _output_get (set `self.IsDrifting` (!= AxisValue 0.0)))
  (if _output_get
    (bind (_true _returnvalue) (`self.Remap_Axis`))
    (`self.K2_SetActorRotation` (`KismetMathLibrary.ComposeRotators` (`self.K2_GetActorRotation`) (`KismetMathLibrary.RotatorFromAxisAndAngle` (`self.GetActorUpVector`) (* _returnvalue (`self.DriftDirection`) AxisValue))))
    ;;;[1 1 0] Setting Nitro
    (`self.SetEnergy`)
    (else
      (set `self.DriftDirection` 0))))

(event `InputAction|Nitro`
  (params (Key :type "Key Structure"))
  ;[1 1 1] Input
  ;;[1 1 0] Nitro
  (:`Pressed`
    (if (`self.CanNitro`)
      (set `self.EnergyBeforeNitro` (`self.Energy`))
      (set `self.isNitro` true)))
  (:`Released`
    (set `self.isNitro` false)
    (`self.Reset Nitro Time`)))

(event `InputAction|Brake`
  (params (Key :type "Key Structure"))
  ;[1 1 1] Input
  ;;[0.4479 0.2305 0] Brake
  (:`Pressed`
    (set `self.isBraking` true))
  (:`Released`
    (set `self.isBraking` false)))

(event `UpdateEvent`
  ;[0 0 0] Not Use
)

(fn `Debug`
  (bind _returnvalue (`self.K2_GetActorLocation`))
  ;[0 1 0] Throttle
  (`KismetSystemLibrary.PrintString` (`KismetTextLibrary.Conv_TextToString` (`|FormatText` "MAXSpeed : { A }   /  Last Speed : {B} / Acc Time : {C}  /  Dec Time: {D} / Acc Curve : {E} / Dec Curve : {F}" (`self.MAXSpeed`) (`self.LastSpeed`) (`self.AccTime`) (`self.DecTime`) (`CurveFloat.GetFloatValue` (`self.AccCurve`) (`self.ScaleAccCurve`)) (`CurveFloat.GetFloatValue` (`self.DecCurve`) (`self.ScaleDecCurve`)))) true true (struct :`G` 1.0 :`A` 1.0))
  ;[1 0 1] Drift
  (`KismetSystemLibrary.PrintString` (`KismetTextLibrary.Conv_TextToString` (`|FormatText` "Drift Direction : { A } / Base Drift Scale { B } / minDriftScale : {C} / MAX DriftScale : { D} / Drift Boost : {E}" (`self.DriftDirection`) (`self.baseDriftScale`) (`self.minDriftScale`) (`self.MAXDriftScale`) (`self.DriftBoosts`))) true true (struct :`R` 1.0 :`B` 1.0 :`A` 1.0))
  ;[1 1 0] Nitro
  (`KismetSystemLibrary.PrintString` (`KismetTextLibrary.Conv_TextToString` (`|FormatText` "Energy : { A } / Number of Jauge {B} / Nitro Boost : {C} / min Gain: {D} / MAX Gain : {E}" (`self.Energy`) (`self.nbNitroJauge`) (`self.NitroSpeed`) (`self.minGainNitro`) (`self.MAXGainNitro`))) true true (struct :`R` 1.0 :`G` 1.0 :`A` 1.0))
  (`KismetSystemLibrary.LineTraceSingle` :`Start` _returnvalue :`End` (+ _returnvalue (* (`KismetMathLibrary.NegateVector` (`self.GetActorUpVector`)) 1000.0)) :`TraceChannel` "TraceTypeQuery1" :`DrawDebugType` (select `bool` (`self.isDebug`) :`true` "ForDuration" :!type "EDrawDebugTrace Enum")))

(fn `Remap_Axis`
  (returns (True :type Boolean) (ReturnValue :type "Float (double-precision)"))
  (bind _returnvalue (`self.GetInputAxisValue`))
  (bind _maxdriftscale (`self.MAXDriftScale`))
  (bind _mindriftscale (`self.minDriftScale`))
  (bind _driftdirection (`self.DriftDirection`))
  (bind _returnvalue_2 (== _driftdirection 1))
  (bind _returnvalue_3 (!= _driftdirection 0))
  (if _returnvalue_3
    (return _returnvalue_3 (select `bool` (!= _returnvalue 0.0) :`false` (`self.baseDriftScale`) :`true` (`KismetMathLibrary.MapRangeClamped` _returnvalue -1.0 1.0 (select `bool` _returnvalue_2 :`false` _maxdriftscale :`true` _mindriftscale) (select `bool` _returnvalue_2 :`false` _mindriftscale :`true` _maxdriftscale))))))

(fn `SetEnergy`
  (returns (NewParam :type Boolean))
  (bind _maxgainnitro (`self.MAXGainNitro`))
  (bind _mingainnitro (`self.minGainNitro`))
  (bind _driftdirection (`self.DriftDirection`))
  (bind _returnvalue (== _driftdirection 1))
  (if (!= _driftdirection 0)
    (bind _output_get (set `self.Energy` (`KismetMathLibrary.FClamp` (+ (`self.Energy`) (`KismetMathLibrary.MapRangeClamped` (`self.GetInputAxisValue`) -1.0 1.0 (select `bool` _returnvalue :`false` _maxgainnitro :`true` _mingainnitro) (select `bool` _returnvalue :`false` _mingainnitro :`true` _maxgainnitro))) 0.0 100.0)))
    (if (> _output_get 0.0)
      (set `self.CanNitro` true))
    (return false)))

(fn `UpdateRotToGround`
  (params (GroundDistance :type "Float (single-precision)") (VectorUp :type "Vector Structure"))
  (returns (NewRotation :type "Rotator Structure"))
  (bind _returnvalue (`self.K2_GetActorLocation`))
  (bind (_outhit _returnvalue_2) (`KismetSystemLibrary.LineTraceSingle` :`Start` _returnvalue :`End` (+ _returnvalue (* (`KismetMathLibrary.NegateVector` VectorUp) GroundDistance)) :`TraceChannel` "TraceTypeQuery1" :`DrawDebugType` (select `bool` (`self.isDebug`) :`true` "ForDuration" :!type "EDrawDebugTrace Enum") :`DrawTime` 0.25))
  (if _returnvalue_2
    (return (`KismetMathLibrary.MakeRotFromXZ` (`KismetMathLibrary.ProjectVectorOnToPlane` (`self.GetActorForwardVector`) (`.Normal` (`GameplayStatics.BreakHitResult` _outhit))) (`.Normal` (`GameplayStatics.BreakHitResult` _outhit))))))

(fn `UserConstructionScript`)